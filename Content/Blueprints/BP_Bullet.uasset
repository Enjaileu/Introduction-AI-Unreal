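; BP_Bullet is a projectile that destroys itself when it hits something and damages what it struck.
; Its Hit event applies damage at the impact point, along the impact normal, to DestructibleActors.
; ThirdPersonCharacters instead lose random Life and get a short lifespan once it runs out.
; Both cases print a hit message whose damage figure is a separate random call, not the damage applied.
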(event `self.ReceiveHit`
  (params (MyComp :type "PrimitiveComponent Object Reference") (Other :type "Actor Object Reference") (OtherComp :type "PrimitiveComponent Object Reference") (bSelfMoved :type Boolean) (HitLocation :type "Vector Structure") (HitNormal :type "Vector Structure") (NormalImpulse :type "Vector Structure") (Hit :type "HitResult Structure (by ref)"))
  (bind (_bblockinghit _binitialoverlap _time _distance _location _impactpoint _normal _impactnormal _physmat _hitactor) (`GameplayStatics.BreakHitResult` Hit))
  (bind _returnvalue (`KismetMathLibrary.RandomFloatInRange` 0.5 3.0))
  (bind _result (`|FormatText` "Hit {actor} - {damages} Damages" (`KismetTextLibrary.Conv_StringToText` (`KismetStringLibrary.Conv_ObjectToString` _hitactor)) _returnvalue))
  (`|ExecutionSequence`
    (:`then_0`
      (`self.K2_DestroyActor`)
      (bind _asdestructible_actor (cast `DestructibleActor` _hitactor))
      (`DestructibleComponent.ApplyDamage` (`DestructibleActor.DestructibleComponent` _asdestructible_actor) 0.0 _impactpoint (* _impactnormal 1.0) 0.0)
      (`KismetSystemLibrary.PrintText` _result))
    (:`then_1`
      (bind _asthird_person_character (cast `/Game/ThirdPersonBP/Blueprints/ThirdPersonCharacter` _hitactor))
      (bind _output_get (set `/Game/ThirdPersonBP/Blueprints/ThirdPersonCharacter.Life` (- (`/Game/ThirdPersonBP/Blueprints/ThirdPersonCharacter.Life` _asthird_person_character) _returnvalue) _asthird_person_character))
      (`KismetSystemLibrary.PrintText` _result)
      (if (<= _output_get 0.0)
        (`self.SetLifeSpan` _asthird_person_character 1.5)))))

(fn `UserConstructionScript`)